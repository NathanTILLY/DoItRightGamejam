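; Base actor for mouse-editable elements whose mesh a visible "mouse" component lifts and sets back down when the player interacts.
; Interact calls DecuTriche on the game instance, lowers Mouse1, attaches it to the mesh, moves both up and back down, then detaches, hides and resets the mouse.
; CollisionOff and CollisionOn switch the mesh's object type between GameTraceChannel1 and WorldStatic.
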(event `CollisionOff`
  (`PrimitiveComponent.SetCollisionObjectType` (`self.StaticMesh`) "ECC_GameTraceChannel1"))

(event `CollisionOn`
  (`PrimitiveComponent.SetCollisionObjectType` (`self.StaticMesh`) "ECC_WorldStatic"))

(event `/Game/Blueprint/BPI_Interact.Interact`
  (params (Player :type "Character Object Reference"))
  (bind _staticmesh (`self.StaticMesh`))
  (bind _mouse1 (`self.Mouse1`))
  (bind _staticmesh_2 (`self.StaticMesh`))
  (bind _mouse1_2 (`self.Mouse1`))
  (bind _returnvalue (`SceneComponent.GetRelativeTransform` _mouse1))
  (bind _returnvalue_2 (`SceneComponent.GetRelativeTransform` _staticmesh_2))
  (bind _returnvalue_3 (`SceneComponent.GetRelativeTransform` _staticmesh))
  (bind _returnvalue_4 (`SceneComponent.GetRelativeTransform` _mouse1_2))
  (cast `/Game/Blueprint/BP_Player` Player)
  (`/Game/Blueprint/BP_GameInstance.DecuTriche` (cast `/Game/Blueprint/BP_GameInstance` (`GameplayStatics.GetGameInstance`) :!pure true))
  (`SceneComponent.SetVisibility` _mouse1_2 true false)
  (`KismetSystemLibrary.MoveComponentTo` _mouse1_2 (`KismetMathLibrary.MakeVector` (.x (.location _returnvalue_4)) (.y (.location _returnvalue_4)) (- (.z (.location _returnvalue_4)) 400.0)) (.rotation _returnvalue_4) false false 3.0)
  (`KismetSystemLibrary.Delay` 1.0)
  (`SceneComponent.K2_AttachToComponent` (`self.Mouse1`) (`self.StaticMesh`) "None" "KeepWorld" "KeepWorld" "KeepWorld" true)
  (`KismetSystemLibrary.MoveComponentTo` _staticmesh (`KismetMathLibrary.MakeVector` (.x (.location _returnvalue_3)) (.y (.location _returnvalue_3)) (+ (.z (.location _returnvalue_3)) 400.0)) (.rotation _returnvalue_3) false false 5.0)
  (`KismetSystemLibrary.MoveComponentTo` _staticmesh_2 (`KismetMathLibrary.MakeVector` (.x (.location _returnvalue_2)) (.y (.location _returnvalue_2)) (- (.z (.location _returnvalue_2)) 400.0)) (.rotation _returnvalue_2) false false 5.0)
  (`SceneComponent.K2_DetachFromComponent` (`self.Mouse1`) "KeepWorld" "KeepWorld" "KeepWorld" true)
  (`SceneComponent.SetVisibility` _mouse1 false false)
  (`KismetSystemLibrary.MoveComponentTo` _mouse1 (`KismetMathLibrary.MakeVector` (.x (.location _returnvalue)) (.y (.location _returnvalue)) (+ (.z (.location _returnvalue)) 400.0)) (.rotation _returnvalue) false false 0.01))

(fn `UserConstructionScript`)